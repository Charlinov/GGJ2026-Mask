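; Shelf interact point, needing no item going by its name, that slides its Box component back and forth along local X when used.
; Interacting starts the push and stopping interaction pauses it.
; Tick moves the box at a constant speed derived from MaxOffset and TimeToMove, printing the offset for debugging.
; Reaching either end halts movement, with direction flipping so the next interaction travels the opposite way.
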(event `self.ReceiveBeginPlay`
  (`parent.ReceiveBeginPlay`)
  (set `self.OffsetPerSecond` (/ (`self.MaxOffset`) (`self.TimeToMove`))))

(event `self.ReceiveTick`
  (params (DeltaSeconds :type "Float (single-precision)"))
  (bind _returnvalue (+ (`self.LocalOffset`) (* DeltaSeconds (`self.OffsetPerSecond`))))
  (bind _returnvalue_2 (- (`self.LocalOffset`) (* DeltaSeconds (`self.OffsetPerSecond`))))
  (`parent.ReceiveTick` DeltaSeconds)
  (if (`self.bIsPushing`)
    (if (`self.bIsReversing`)
      (if (<= _returnvalue_2 0.0)
        (set `self.bIsReversing` false)
        (set `self.bIsPushing` false)
        (else
          (bind _output_get (set `self.LocalOffset` (`KismetMathLibrary.FClamp` _returnvalue_2 -30.0 (`self.MaxOffset`))))
          (`KismetSystemLibrary.PrintString` (`KismetStringLibrary.Conv_DoubleToString` _output_get))
          (`SceneComponent.K2_SetRelativeLocation` (`self.Box`) (`KismetMathLibrary.MakeVector` _output_get 0.0 78.0) false false)))
      (elif (>= _returnvalue (`self.MaxOffset`))
        (set `self.bIsReversing` true)
        (set `self.bIsPushing` false)
        (else
          (bind _output_get_2 (set `self.LocalOffset` (`KismetMathLibrary.FClamp` _returnvalue -30.0 (`self.MaxOffset`))))
          (`KismetSystemLibrary.PrintString` (`KismetStringLibrary.Conv_DoubleToString` _output_get_2))
          (`SceneComponent.K2_SetRelativeLocation` (`self.Box`) (`KismetMathLibrary.MakeVector` _output_get_2 0.0 78.0) false false))))))

(fn `InteractWithPoint`
  (returns (ShouldContinue :type Boolean))
  (bind _shouldcontinue (`parent.InteractWithPoint`))
  (set `self.bIsPushing` true)
  (return _shouldcontinue))

(fn `StopInteractWithItem`
  (`parent.StopInteractWithItem`)
  (set `self.bIsPushing` false))

(fn `UserConstructionScript`
  (`parent.UserConstructionScript`))