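; Door interact point Blueprint that ends the game in victory when the player uses it while holding the required item.
; Its InteractWithPoint override gets the first-person character and checks whether its HeldItem matches the AllowedHeldItem class.
; On a match it shows the victory screen widget, enables the mouse cursor and switches input to UI only.
; The parent InteractWithPoint call is left unconnected, so base behavior never runs.
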(fn `InteractWithPoint`
  (returns (ShouldContinue :type Boolean))
  (bind _returnvalue (`GameplayStatics.GetPlayerController` 0))
  (bind _asbp_first_person_character (cast `/Game/FirstPerson/Blueprints/BP_FirstPersonCharacter` (`GameplayStatics.GetPlayerCharacter` 0)))
  (if (`GameplayStatics.ObjectIsA` (`/Game/FirstPerson/Blueprints/BP_FirstPersonCharacter.HeldItem` _asbp_first_person_character) (`self.AllowedHeldItem`))
    (bind _returnvalue_2 (`|CreateWidget` "/Game/UI/WBP_VictoryScreen.WBP_VictoryScreen_C" (`GameplayStatics.GetPlayerController` 0)))
    (`UserWidget.AddToViewport` _returnvalue_2 0)
    (set `PlayerController.bShowMouseCursor` true _returnvalue)
    (`WidgetBlueprintLibrary.SetInputMode_UIOnlyEx` _returnvalue null)))

(fn `UserConstructionScript`
  (`parent.UserConstructionScript`))