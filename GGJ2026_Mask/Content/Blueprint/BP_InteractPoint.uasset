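; BP_InteractPoint is a world interaction point that toggles or sets a Disturbed state and can hold one item of an allowed class.
; Tick turns its prompt widget toward the player, showing and scaling it by distance, and accumulates hold time.
; Instant interactions toggle Disturbed, completed holds set it, and NeverDisturb clears it every frame.
; Hover sends progress to the character's HUD, while TryDropItem snaps items to a socket.
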(event `self.ReceiveBeginPlay`
  (bind _nextinteract (`self.NextInteract`))
  (`/Engine/EditorBlueprintResources/StandardMacros.IsValid` _nextinteract
    (:`Is Valid`
      (`SceneComponent.SetVisibility` (`/Game/Blueprint/BP_InteractPoint.Widget` _nextinteract) false false))))

(event `self.ReceiveTick`
  (params (DeltaSeconds :type "Float (single-precision)"))
  (bind _widget (`self.Widget`))
  (bind _widget_2 (`self.Widget`))
  (bind _returnvalue (`self.K2_GetActorLocation` (`GameplayStatics.GetPlayerCharacter` 0)))
  (bind _returnvalue_2 (`SceneComponent.K2_GetComponentLocation` _widget))
  (bind _returnvalue_3 (`KismetMathLibrary.Vector_Distance` _returnvalue_2 _returnvalue))
  (bind _returnvalue_4 (`KismetMathLibrary.MapRangeClamped` _returnvalue_3 100.0 300.0 0.03 0.05))
  (`|ExecutionSequence`
    (:`then_0`
      (if (`self.bCanInteract`)
        (`SceneComponent.K2_SetWorldRotation` _widget (`KismetMathLibrary.FindLookAtRotation` _returnvalue_2 _returnvalue) false false)
        (if (< _returnvalue_3 300.0)
          (`SceneComponent.SetVisibility` _widget_2 true false)
          (`SceneComponent.SetWorldScale3D` _widget_2 (`KismetMathLibrary.MakeVector` _returnvalue_4 _returnvalue_4 _returnvalue_4))
          (else
            (`SceneComponent.SetVisibility` _widget_2 false false)))))
    (:`then_1`
      (if (`self.bMustHold`)
        (if (`self.bInteracting`)
          (bind _output_get (set `self.holdTimer` (+ (`self.holdTimer`) DeltaSeconds)))
          (if (>= _output_get (`self.holdTime`))
            (`self.FinishInteract`)))))
    (:`then_2`
      (if (`self.bNeverDisturb`)
        (set `self.bDisturbed` false)))))

(event `Hover`
  (if (`self.bMustHold`)
    (bind _asbp_first_person_character (cast `/Game/FirstPerson/Blueprints/BP_FirstPersonCharacter` (`GameplayStatics.GetPlayerCharacter` 0)))
    (`/Game/FirstPerson/Blueprints/BP_FirstPersonCharacter.SetHudProgress` _asbp_first_person_character (/ (`self.holdTimer`) (`self.holdTime`)))
    (else
      (bind _asbp_first_person_character_2 (cast `/Game/FirstPerson/Blueprints/BP_FirstPersonCharacter` (`GameplayStatics.GetPlayerCharacter` 0)))
      (`/Game/FirstPerson/Blueprints/BP_FirstPersonCharacter.SetHudProgress` _asbp_first_person_character_2 1.0))))

(event `Interact`)

(fn `FinishInteract`
  (set `self.bDisturbed` true))

(fn `GetHeldItem`
  (returns (NewParam :type "/Game/Blueprint/BP_PuzzleItem Object Reference"))
  (locals (HeldItemRef :type "/Game/Blueprint/BP_PuzzleItem Object Reference"))
  (bind _output_get (set `local.HeldItemRef` (`self.HeldItem`)))
  (set `self.HeldItem` null)
  (return _output_get))

(fn `InteractWithPoint`
  (returns (ShouldContinue :type Boolean))
  (if (`self.bCanInteract`)
    (set `self.bInteracting` true)
    (if (not (`self.bMustHold`))
      (set `self.bDisturbed` (not (`self.bDisturbed`))))
    (return true)
    (else
      (return false))))

(fn `StopInteractWithItem`
  (set `self.bInteracting` false))

(fn `TryDropItem`
  (params (ItemToDrop :type "/Game/Blueprint/BP_PuzzleItem Object Reference"))
  (returns (NewParam :type Boolean))
  (bind _itemholdsocket (`self.ItemHoldSocket`))
  (`/Engine/EditorBlueprintResources/StandardMacros.IsValid` (`self.HeldItem`)
    (:`Is Valid`
      (return false))
    (:`Is Not Valid`
      (if (`GameplayStatics.ObjectIsA` ItemToDrop (`self.AllowedHeldItem`))
        (bind _output_get (set `self.HeldItem` ItemToDrop))
        (`self.K2_SetActorLocationAndRotation` _output_get (`SceneComponent.K2_GetComponentLocation` _itemholdsocket) (`SceneComponent.K2_GetComponentRotation` _itemholdsocket) false true)
        (`/Game/Blueprint/BP_PuzzleItem.Drop` (`self.HeldItem`))
        (return true)
        (else
          (return false))))))

(fn `UserConstructionScript`)