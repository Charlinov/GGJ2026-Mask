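; BP_Watch is an analog watch that visualizes the progress of a timed session.
; While CanTime is set, Tick accumulates SessionTimer and divides it by SessionTime.
; That ratio drives clamped range mappings that pitch MinuteHand through one full turn and HourHand through one hour mark, from a configurable start offset, so a session reads as one hour.
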(event `self.ReceiveTick`
  (params (DeltaSeconds :type "Float (single-precision)"))
  (bind _returnvalue (/ (`self.SessionTimer`) (`self.SessionTime`)))
  (if (`self.CanTime`)
    (set `self.SessionTimer` (+ DeltaSeconds (`self.SessionTimer`)))
    (`SceneComponent.K2_SetRelativeRotation` (`self.Minute Hand`) (`KismetMathLibrary.MakeRotator` 180.0 (+ 90.0 (`KismetMathLibrary.MapRangeClamped` _returnvalue 0.0 1.0 0.0 360.0)) 180.0) false false)
    (`SceneComponent.K2_SetRelativeRotation` (`self.Hour Hand`) (`KismetMathLibrary.MakeRotator` 180.0 (+ (+ (`self.HourHandStartOffset`) -20.0) (`KismetMathLibrary.MapRangeClamped` _returnvalue 0.0 1.0 0.0 30.0)) 180.0) false false)))

(fn `UserConstructionScript`)