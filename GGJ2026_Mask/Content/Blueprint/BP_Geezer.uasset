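; BP_Geezer is an actor Blueprint for a skeletal-mesh character that tracks whether it is moving.
; BeginPlay caches the mesh's world location, then each Tick compares the current location to that cached value, sets IsMoving and updates the cache.
; Any nonzero displacement counts as movement, with no threshold or velocity query.
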(event `self.ReceiveBeginPlay`
  (set `self.LastPos` (`SceneComponent.K2_GetComponentLocation` (`self.SkeletalMesh`))))

(event `self.ReceiveTick`
  (params (DeltaSeconds :type "Float (single-precision)"))
  (bind _returnvalue (`SceneComponent.K2_GetComponentLocation` (`self.SkeletalMesh`)))
  (set `self.bIsMoving` (> (`KismetMathLibrary.VSize` (- _returnvalue (`self.LastPos`))) 0.0))
  (set `self.LastPos` _returnvalue))

(fn `UserConstructionScript`)