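; An interaction point where a held item, by name resin, melts into a key while the furnace is lit.
; On BeginPlay it finds the furnace actor in the level.
; Tick accumulates melt time while an item is held and the fire is on, then replaces the item with a key spawned at the hold socket.
; The timer never resets here and item type is unchecked, so replacement repeats each qualifying tick afterwards.
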(event `self.ReceiveBeginPlay`
  (`parent.ReceiveBeginPlay`)
  (bind _returnvalue (`GameplayStatics.GetActorOfClass` "/Game/Blueprint/BP_InteractPoint_Furnace.BP_InteractPoint_Furnace_C"))
  (set `self.Furnace` _returnvalue))

(event `self.ReceiveTick`
  (params (DeltaSeconds :type "Float (single-precision)"))
  (bind (_returnvalue_location _returnvalue_rotation) (`KismetMathLibrary.BreakTransform` (`SceneComponent.K2_GetComponentToWorld` (`self.ItemHoldSocket`))))
  (`parent.ReceiveTick` DeltaSeconds)
  (`/Engine/EditorBlueprintResources/StandardMacros.IsValid` (`self.HeldItem`)
    (:`Is Valid`
      (if (`/Game/Blueprint/BP_InteractPoint_Furnace.bFireOn` (`self.Furnace`))
        (bind _output_get (set `self.resinMeltTimer` (+ (`self.resinMeltTimer`) DeltaSeconds)))
        (if (>= _output_get (`self.resinMeltTime`))
          (`self.K2_DestroyActor` (`self.HeldItem`))
          (bind _returnvalue (`|SpawnActorFromClass` "/Game/Blueprint/BP_HoldableItem_Key.BP_HoldableItem_Key_C" (`KismetMathLibrary.MakeTransform` _returnvalue_location _returnvalue_rotation) "Undefined" "MultiplyWithRoot" null null))
          (set `self.HeldItem` _returnvalue))))))

(fn `UserConstructionScript`
  (`parent.UserConstructionScript`))