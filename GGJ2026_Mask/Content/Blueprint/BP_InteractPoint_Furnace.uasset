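; Furnace interact point that the player loads with logs, lights with a matchbox, or otherwise opens and closes by rotating its door.
; Allowed items reveal up to three log meshes while Disturbed is set, which also gates item drops through the parent.
; With all logs deposited, the matchbox shows the fire, swaps logs to burned material and sets FireOn.
; Tick clears the point's HeldItem every frame.
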(event `self.ReceiveTick`
  (params (DeltaSeconds :type "Float (single-precision)"))
  (`parent.ReceiveTick` DeltaSeconds)
  (set `self.HeldItem` null))

(fn `InteractWithPoint`
  (returns (ShouldContinue :type Boolean))
  (bind _furance_door (`self.Furance_Door`))
  (bind _asbp_first_person_character (cast `/Game/FirstPerson/Blueprints/BP_FirstPersonCharacter` (`GameplayStatics.GetPlayerCharacter` 0)))
  (bind _helditem (`/Game/FirstPerson/Blueprints/BP_FirstPersonCharacter.HeldItem` _asbp_first_person_character))
  (if (`GameplayStatics.ObjectIsA` _helditem (`self.AllowedHeldItem`))
    (if (`self.bDisturbed`)
      (switch `int` (`self.LogsDeposited`)
        (:`0`
          (`SceneComponent.SetVisibility` (`self.Log`) true false))
        (:`1`
          (`SceneComponent.SetVisibility` (`self.Log1`) true false))
        (:`2`
          (`SceneComponent.SetVisibility` (`self.Log2`) true false)))
      (bind _result (`/Engine/EditorBlueprintResources/StandardMacros.IncrementInt` (`self.LogsDeposited`))
        (:`  `
          (set `self.LogsDeposited` _result))))
    (elif (`GameplayStatics.ObjectIsA` _helditem "/Game/Blueprint/BP_HoldableItem_MatchBox.BP_HoldableItem_MatchBox_C")
      (if (> (`self.LogsDeposited`) 2)
        (`SceneComponent.SetVisibility` (`self.Fire`) true false)
        (`PrimitiveComponent.SetMaterial` (`self.Log1`) 0 "/Game/LogCabin/Materials/Instances/Props/MI_Log_01_Burned.MI_Log_01_Burned")
        (`PrimitiveComponent.SetMaterial` (`self.Log`) 0 "/Game/LogCabin/Materials/Instances/Props/MI_Log_01_Burned.MI_Log_01_Burned")
        (`PrimitiveComponent.SetMaterial` (`self.Log2`) 0 "/Game/LogCabin/Materials/Instances/Props/MI_Log_01_Burned.MI_Log_01_Burned")
        (set `self.bFireOn` true))
      (else
        ; Open/Close
        (if (`self.bDisturbed`)
          (`SceneComponent.K2_SetRelativeRotation` :`self` _furance_door)
          (else
            (`SceneComponent.K2_SetRelativeRotation` _furance_door (struct :`Yaw` 90.0) false false)))
        (bind _shouldcontinue (`parent.InteractWithPoint`))
        (return _shouldcontinue)))))

(fn `TryDropItem`
  (params (ItemToDrop :type "/Game/Blueprint/BP_PuzzleItem Object Reference"))
  (returns (NewParam :type Boolean))
  (if (`self.bDisturbed`)
    (bind _newparam (`parent.TryDropItem` ItemToDrop))
    (return _newparam)
    (else
      (return false))))

(fn `UserConstructionScript`
  (`parent.UserConstructionScript`))